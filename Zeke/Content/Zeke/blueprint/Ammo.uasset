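; Ammo projectile Blueprint in a test state, launched by a physics impulse when it spawns.
; BeginPlay scales the sum of actor location, forward vector and AmmoOffset by AmmoVelocity, so the impulse depends on world position as well as facing.
; Hit and AmmoDamage end-overlap events are empty.
; Damage, alternative impulse and move-to nodes are left disconnected, so the ammo currently deals no damage.
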(event `self.ReceiveBeginPlay`
  ;[1 1 1] Testing shooting stuff
  (`PrimitiveComponent.AddImpulse` (* (+ (`self.K2_GetActorLocation`) (`KismetMathLibrary.Conv_RotatorToVector` (`self.K2_GetActorRotation`)) (`self.Ammo Offset`)) (`self.Ammo Velocity`))))

(event `self.ReceiveHit`
  (params (MyComp :type "PrimitiveComponent Object Reference") (Other :type "Actor Object Reference") (OtherComp :type "PrimitiveComponent Object Reference") (bSelfMoved :type Boolean) (HitLocation :type "Object.Vector Structure") (HitNormal :type "Object.Vector Structure") (NormalImpulse :type "Object.Vector Structure") (Hit :type "EngineTypes.HitResult Structure (by ref)")))

(event `self.AmmoDamage.OnComponentEndOverlap`
  (params (OtherActor :type "Actor Object Reference") (OtherComp :type "PrimitiveComponent Object Reference") (OtherBodyIndex :type Integer))
  ;[1 1 1] Does damage to character
)

(fn `UserConstructionScript`)