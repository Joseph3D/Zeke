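; Pistol actor that spawns an Ammo actor when something begins overlapping its ShootPlayer component, apparently to fire at the player.
; The spawn point is the pistol's location plus PistolOffset, without its rotation, and ignores collisions.
; The AddImpulse launch using AmmoVelocity, along with DoOnce and Delay nodes, is disconnected, so ammo gets no impulse here; the author notes shooting is broken.
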(event `self.ShootPlayer.OnComponentBeginOverlap`
  (params (OtherActor :type "Actor Object Reference") (OtherComp :type "PrimitiveComponent Object Reference") (OtherBodyIndex :type Integer) (bFromSweep :type Boolean) (SweepResult :type "EngineTypes.HitResult Structure (by ref)"))
  ;[1 1 1] Makes ammo shoot (Doesnt work properly)
  (bind _returnvalue (`|SpawnActorFromClass` "/Game/Zeke/blueprint/Ammo.Ammo_C" (`KismetMathLibrary.Conv_VectorToTransform` (+ (.location (`self.GetTransform`)) (`self.PistolOffset`))) true)))

(fn `UserConstructionScript`)